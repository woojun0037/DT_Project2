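; BP_SplineObject is an actor that moves a configurable mesh along the spline of a referenced SplineToFollow.
; The construction script applies ObjectMesh to the Cube component, and BeginPlay calls MoveObject.
; A timeline, with play rate scaled by TimeToComplete, lerps distance over the spline length to set world location and local-space spline rotation on the actor.
; An invalid spline reference prints a red error instead.
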(event `self.ReceiveBeginPlay`
  (`self.MoveObject`))

(event `MoveObject`
  (bind _spline_to_follow (`self.Spline To Follow`))
  (bind _spline (`/Game/BP/Rail/BP_ModularRail.Spline` _spline_to_follow))
  (`/Engine/EditorBlueprintResources/StandardMacros.IsValid` _spline_to_follow
    (:`Is Valid`
      (`TimelineComponent.SetPlayRate` (`self.T_Move`) (/ 1.0 (`self.Time To Complete`)))
      (bind (_direction _move_track) (`Timeline|T_Move`)
        (:`Update`
          (bind _returnvalue (`KismetMathLibrary.Lerp` 0.0 (`SplineComponent.GetSplineLength` _spline) _move_track))
          (`self.K2_SetActorLocationAndRotation` (`SplineComponent.GetLocationAtDistanceAlongSpline` _spline _returnvalue "World") (`SplineComponent.GetRotationAtDistanceAlongSpline` _spline _returnvalue "Local")))))
    (:`Is Not Valid`
      (`KismetSystemLibrary.PrintString` "Invalid \"Spline to Follow\"" true true (struct :`R` 1.0 :`A` 1.0)))))

(fn `UserConstructionScript`
  (`StaticMeshComponent.SetStaticMesh` (`self.Cube`) (`self.ObjectMesh`)))