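; Modular rail actor that lays a rail mesh along a spline and destroys any BP_MyBox that enters its box trigger.
; When enabled by a flag, the Construction Script rebuilds Instanced Static Mesh instances at SegmentLength intervals along the spline.
; A disconnected spline-mesh alternative remains, with start/end tangent helpers; the end helper ignores its index.
; An author note says generation works but not as intended.
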(event `self.Box.OnComponentBeginOverlap`
  (params (OverlappedComponent :type "PrimitiveComponent Object Reference") (OtherActor :type "Actor Object Reference") (OtherComp :type "PrimitiveComponent Object Reference") (OtherBodyIndex :type Integer) (bFromSweep :type Boolean) (SweepResult :type "HitResult Structure (by ref)"))
  (bind _asbp_my_box (cast `/Game/BP/Spawner/BP_MyBox` OtherActor))
  (`self.K2_DestroyActor` _asbp_my_box)
  (`KismetSystemLibrary.PrintString` "Destroy" true true (struct :`R` 1.0 :`A` 1.0)))

(fn `Get EndPosTangent`
  (params (Index :type Integer))
  (returns (Position :type "Vector Structure") (Target :type "Vector Structure"))
  (bind _spline (`self.Spline`))
  (bind _returnvalue (* (/ 0 1) (`self.SectionLength`)))
  (return (`SplineComponent.GetLocationAtDistanceAlongSpline` _spline _returnvalue "Local") (`KismetMathLibrary.ClampVectorSize` (`SplineComponent.GetLocationAtDistanceAlongSpline` _spline _returnvalue "Local") 0.0 (`self.SectionLength`))))

(fn `Get Start PosTangent`
  (params (Index :type Integer))
  (returns (Position :type "Vector Structure") (Tangent :type "Vector Structure"))
  (bind _spline (`self.Spline`))
  (bind _returnvalue (* Index (`self.SectionLength`)))
  (return (`SplineComponent.GetLocationAtDistanceAlongSpline` _spline _returnvalue "Local") (`KismetMathLibrary.ClampVectorSize` (`SplineComponent.GetLocationAtDistanceAlongSpline` _spline _returnvalue "Local") 0.0 (`self.SectionLength`))))

(fn `UserConstructionScript`
  (bind _instancedstaticmesh (`self.InstancedStaticMesh`))
  ; 레일 생성은 됨 근데 원하는대로 안됨
  (if (`self.bConstructionScript`)
    (`KismetSystemLibrary.PrintString` "Construction Script")
    (`StaticMeshComponent.SetStaticMesh` _instancedstaticmesh (`self.RailMesh`))
    (`InstancedStaticMeshComponent.ClearInstances` _instancedstaticmesh)
    (for _index (range (+ (`KismetMathLibrary.Max` (- (`KismetMathLibrary.FFloor` (/ (`SplineComponent.GetSplineLength` (`self.Spline`)) (`self.SegmentLength`))) 1)) 1))
      (`InstancedStaticMeshComponent.AddInstance` _instancedstaticmesh (`SplineComponent.GetTransformAtDistanceAlongSpline` (`self.Spline`) (* _index (`self.SegmentLength`)) "Local" false) false))))