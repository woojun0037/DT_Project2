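; Box spawner actor that creates one box at the first point of a spline path on BeginPlay and moves it along a spline.
; Spawn finds the first BP_MySpline and passes it to the new box, with class and config drawn randomly from SpawnDataList.
; Tick advances a distance by SpeedOnSpline and sets the box mesh's transform from a separate SplineTransfom reference, which is not assigned in these graphs.
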(event `Spawn`
  (bind (_boxtypeinfo _boxbpclass) (break `/Game/BP/BoxData/ST_BoxSpawnData` (`KismetArrayLibrary.Array_Random` (`self.SpawnDataList`))))
  (bind _outactors (`GameplayStatics.GetAllActorsOfClass` "/Game/BP/Spline/BP_MySpline.BP_MySpline_C"))
  (if (`KismetArrayLibrary.Array_IsNotEmpty` _outactors)
    (bind _output (`|GetArrayItem` _outactors))
    (bind _returnvalue (`|SpawnActorFromClass` _boxbpclass (`SplineComponent.GetTransformAtSplinePoint` (`/Game/BP/Spline/BP_MySpline.PathSpline` _output) 0 "World" false) "Undefined" "MultiplyWithRoot" (`self.BP_Box`) _boxtypeinfo _output null))
    (set `self.BP_Box` _returnvalue)))

(event `self.ReceiveBeginPlay`
  (`self.Spawn`))

(event `self.ReceiveTick`
  (params (DeltaSeconds :type "Float (single-precision)"))
  (bind _output_get (set `self.Position On Spline` (+ (* DeltaSeconds (`self.Speed On Spline`)) (`self.Position On Spline`))))
  (`SceneComponent.K2_SetWorldTransform` (`/Game/BP/Box/BP_Box.StaticMesh` (`self.BP_Box`)) (`SplineComponent.GetTransformAtDistanceAlongSpline` (`/Game/BP/Spline/BP_MySpline.PathSpline` (`self.SplineTransfom`)) _output_get "World" false) false false))

(fn `NewFunction`
  (returns (OutItem :type "/Game/BP/BoxData/ST_BoxSpawnData Structure"))
  (return (`KismetArrayLibrary.Array_Random` (`self.SpawnDataList`))))

(fn `UserConstructionScript`)