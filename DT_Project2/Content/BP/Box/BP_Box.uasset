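; BP_Box is a configurable box actor that builds its look from a BoxConfig struct on BeginPlay.
; It sets a cube mesh, colors it through a dynamic material instance, and scales it by dividing the configured size by the mesh's local bounds difference (Min minus Max).
; A configured spline actor is cast to BP_MySpline but not used further, and the SplineMovementTimeLine is unconnected, so the box has no movement logic.
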(event `self.ReceiveBeginPlay`
  (bind _boxconfig_boxcolor (break `/Game/BP/BoxData/ST_BoxInfo` (`self.BoxConfig`)))
  (bind (_boxconfig_boxcolor_2 _boxconfig_boxsize) (break `/Game/BP/BoxData/ST_BoxInfo` (`self.BoxConfig`)))
  (bind (_boxconfig_boxcolor_3 _boxconfig_boxsize_2 _boxconfig_splineactorreference) (break `/Game/BP/BoxData/ST_BoxInfo` (`self.BoxConfig`)))
  (bind (_boxconfig_boxcolor_4 _boxconfig_boxsize_3 _boxconfig_splineactorreference_2) (break `/Game/BP/BoxData/ST_BoxInfo` (`self.BoxConfig`)))
  (bind (_min _max) (`StaticMeshComponent.GetLocalBounds` (`self.StaticMesh`)))
  (`StaticMeshComponent.SetStaticMesh` (`self.StaticMesh`) "/Game/StarterContent/Shapes/Shape_Cube.Shape_Cube")
  (`PrimitiveComponent.CreateDynamicMaterialInstance` (`self.StaticMesh`) 0 null "None")
  (bind _output_get (set `self.DynamicBoxMatarial` (`self.DynamicBoxMatarial`)))
  (`MaterialInstanceDynamic.SetVectorParameterValue` _output_get "BaseColor" _boxconfig_boxcolor)
  (bind _output_get_2 (set `self.InitialMeshSize` (* (/ (- _min _max) (2.0 2.0 2.0)) (2.0 2.0 2.0))))
  (`SceneComponent.SetWorldScale3D` (`self.StaticMesh`) (/ _boxconfig_boxsize _output_get_2))
  (if (`KismetSystemLibrary.IsValid` _boxconfig_splineactorreference_2)
    (cast `/Game/BP/Spline/BP_MySpline` _boxconfig_splineactorreference)))

(fn `UserConstructionScript`)