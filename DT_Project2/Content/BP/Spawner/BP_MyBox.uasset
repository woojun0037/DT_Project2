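; BP_MyBox is a spawner box actor that travels along an assigned spline.
; On BeginPlay it colors its mesh through a dynamic material, using the BoxType entry in the GameState's BoxDataMap.
; Tick advances its location by BoxSpeed, while MoveObject separately drives location and rotation with a timeline scaled by TimeToComplete.
; An overlap handler disables collision on the spline actor's MLineConnerL; box scaling is left disconnected.
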(event `self.ReceiveBeginPlay`
  (bind _staticmesh (`self.StaticMesh`))
  (`|ExecutionSequence`
    (:`then_0`
      (bind _asbp_game_state (cast `/Game/BP/Game/BP_GameState` (`GameplayStatics.GetGameState`)))
      (bind _returnvalue (`PrimitiveComponent.CreateDynamicMaterialInstance` _staticmesh 0 (`PrimitiveComponent.GetMaterial` _staticmesh 0) "None"))
      (`MaterialInstanceDynamic.SetVectorParameterValue` _returnvalue "Color" (`.BoxColor_9_C613D54F441A6E118E951FB749CB9BBD` (break `/Game/BP/Spawner/ST_BoxInfo` (`BlueprintMapLibrary.Map_Find` (`/Game/BP/Game/BP_GameState.BoxDataMap` _asbp_game_state) (`self.BoxType`))))))))

(event `OnComponentBeginOverlap_Event`
  (params (OverlappedComponent :type "PrimitiveComponent Object Reference") (OtherActor :type "Actor Object Reference") (OtherComp :type "PrimitiveComponent Object Reference") (OtherBodyIndex :type Integer) (bFromSweep :type Boolean) (SweepResult :type "HitResult Structure (by ref)"))
  (`PrimitiveComponent.SetCollisionEnabled` (`/Game/BP/Rail/BP_ModularRail.M_LineConner_L` (`self.Spline To Follow`)) "NoCollision"))

(event `self.ReceiveTick`
  (params (DeltaSeconds :type "Float (single-precision)"))
  (bind _output_get (set `self.CurrentSplineDistance` (+ (`self.CurrentSplineDistance`) (* DeltaSeconds (`self.BoxSpeed`)))))
  (`self.K2_SetActorLocation` self (`SplineComponent.GetLocationAtDistanceAlongSpline` (`/Game/BP/Rail/BP_ModularRail.Spline` (`self.Spline To Follow`)) _output_get "World") false false))

(event `MoveObject`
  (bind _spline (`/Game/BP/Rail/BP_ModularRail.Spline` (`self.Spline To Follow`)))
  (`/Engine/EditorBlueprintResources/StandardMacros.IsValid` (`self.Spline To Follow`)
    (:`Is Valid`
      (`TimelineComponent.SetPlayRate` (`self.TMove`) (/ 1.0 (`self.TimeToComplete`)))
      (bind (_direction _move_track) (`Timeline|TMove`)
        (:`Update`
          (bind _returnvalue (`KismetMathLibrary.Lerp` 0.0 (`SplineComponent.GetSplineLength` _spline) _move_track))
          (`self.K2_SetActorLocationAndRotation` (`SplineComponent.GetLocationAtDistanceAlongSpline` _spline _returnvalue "World") (`SplineComponent.GetRotationAtDistanceAlongSpline` _spline _returnvalue "World")))))
    (:`Is Not Valid`
      (`KismetSystemLibrary.PrintString` "Invalid \"Spline to Follow\"" true true (struct :`R` 1.0 :`A` 1.0)))))

(fn `SetSplineFollow`
  (params (`Spline To Follow` :type "/Game/BP/Rail/BP_ModularRail Object Reference"))
  (set `self.Spline To Follow` `Spline To Follow`))

(fn `UserConstructionScript`)