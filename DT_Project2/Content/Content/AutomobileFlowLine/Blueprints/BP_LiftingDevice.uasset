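; BP_LiftingDevice is a lifting device for the automobile flow line that moves vertically and can carry a car.
; MoveSettings sets the move flag and signed speed, attaches a valid car to the device keeping world transform, and records whether the direction is upward.
; Tick applies the speed as a per-frame local Z offset, stopping and snapping at a fixed lower height; no upper limit is checked here.
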(event `self.ReceiveTick`
  (params (DeltaSeconds :type "Float (single-precision)"))
  (bind (_returnvalue_x _returnvalue_y _returnvalue_z) (`KismetMathLibrary.BreakVector` (`self.K2_GetActorLocation`)))
  (if (`self.Move?`)
    (`self.K2_AddActorLocalOffset` (`KismetMathLibrary.MakeVector` 0.0 0.0 (`self.MoveSpeed`)))
    (if (< _returnvalue_z 57.260681)
      (set `self.Move?` false)
      (`self.K2_SetActorLocation` (`KismetMathLibrary.MakeVector` _returnvalue_x _returnvalue_y 57.260681)))))

(fn `MoveSettings`
  (params (Move :type Boolean :default true) (MoveSpeed :type "Float (double-precision)" :default 2.0) (BP_Car :type "/Game/AutomobileFlowLine/Blueprints/BP_Car Object Reference"))
  (set `self.Move?` Move)
  (set `self.MoveSpeed` MoveSpeed)
  (set `self.BP_Car` BP_Car)
  (`|ExecutionSequence`
    (:`then_0`
      (bind _bp_car (`self.BP_Car`)
        (:`then`
          (`self.K2_AttachToActor` _bp_car self "None" "KeepWorld" "KeepWorld" "KeepWorld" true))
        (:`else`)))
    (:`then_1`
      (if (> (`self.MoveSpeed`) 0.0)
        (set `self.MovingDirection` true)
        (else
          (set `self.MovingDirection` false))))))

(fn `UserConstructionScript`)