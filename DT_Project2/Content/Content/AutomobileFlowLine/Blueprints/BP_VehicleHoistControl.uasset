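; BP_VehicleHoistControl is a hoist station in the automobile flow line that stops an arriving car and starts its hoist.
; A BP_Car overlapping the Box is stored and starts CE_Parking, which re-calls itself after short delays until the car's Y reaches the actor's own.
; It then halts the car and, after a pause, tells HoistMesh to move with that car.
; BeginPlay also shows the mouse cursor.
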(event `self.ReceiveBeginPlay`
  (set `PlayerController.bShowMouseCursor` true (`GameplayStatics.GetPlayerController` 0)))

(event `CE_Parking`
  (bind (_returnvalue_x _returnvalue_y) (`KismetMathLibrary.BreakVector` (`self.K2_GetActorLocation`)))
  (bind (_returnvalue_x_2 _returnvalue_y_2) (`KismetMathLibrary.BreakVector` (`self.K2_GetActorLocation` (`self.BP_Car`))))
  (`KismetSystemLibrary.Delay` 0.02)
  (if (>= _returnvalue_y_2 _returnvalue_y)
    (set `/Game/AutomobileFlowLine/Blueprints/BP_Car.Move?` false (`self.BP_Car`))
    (`KismetSystemLibrary.Delay` 1.0)
    (`self.HoistMesh`
      (:`then`
        (`/Game/AutomobileFlowLine/Blueprints/BP_LiftingDevice.MoveSettings` (`self.HoistMesh`) true 1.5 (`self.BP_Car`)))
      (:`else`))
    (else
      (`self.CE_Parking`))))

(event `self.Box.OnComponentBeginOverlap`
  (params (OverlappedComponent :type "PrimitiveComponent Object Reference") (OtherActor :type "Actor Object Reference") (OtherComp :type "PrimitiveComponent Object Reference") (OtherBodyIndex :type Integer) (bFromSweep :type Boolean) (SweepResult :type "HitResult Structure (by ref)"))
  (bind _asbp_car (cast `/Game/AutomobileFlowLine/Blueprints/BP_Car` OtherActor))
  (set `self.BP_Car` _asbp_car)
  (`self.CE_Parking`))

(fn `UserConstructionScript`)